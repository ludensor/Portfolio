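; BP_TriangleTessellation is an actor that visualizes and tests the EQ_TriangleTessellation environment query.
; A looping timer started on BeginPlay periodically runs the query in AllMatching mode with the actor as querier.
; When it finishes, every result location gets a short-lived debug sphere.
; It then shuffles the locations and spawns pooled explosion emitters at up to Count of them.
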(event `self.ReceiveBeginPlay`
  (`KismetSystemLibrary.K2_SetTimerDelegate` (delegate `RunQuery`) 3.0 true))

(event `RunQuery`
  (bind _returnvalue (`EnvQueryManager.RunEQSQuery` "/Game/Blueprints/AI/EnvironmentQuery/EQ_TriangleTessellation.EQ_TriangleTessellation" self "AllMatching"))
  (add `EnvQueryInstanceBlueprintWrapper.OnQueryFinishedEvent` _returnvalue (delegate `OnQueryFinished`)))

(event `OnQueryFinished`
  (params (QueryInstance :type "EnvQueryInstanceBlueprintWrapper Object Reference") (QueryStatus :type "EEnvQueryStatus Enum" :default "Processing"))
  (bind _resultlocations (`EnvQueryInstanceBlueprintWrapper.GetQueryResultsAsLocations` QueryInstance))
  (for _array_element _resultlocations
    (`KismetSystemLibrary.DrawDebugSphere` _array_element 16.0 12 (struct :`R` 0.066385 :`G` 0.151396 :`B` 1.0 :`A` 1.0) 3.0))
  (`KismetArrayLibrary.Array_Shuffle` _resultlocations)
  (for _index (range (`KismetMathLibrary.Min` (`KismetArrayLibrary.Array_Length` _resultlocations) (`self.Count`)))
    (`GameplayStatics.SpawnEmitterAtLocation` "/Game/Effects/P_Explosion.P_Explosion" (`|GetArrayItem` _resultlocations _index) (struct) (1.0 1.0 1.0) true "AutoRelease")))

(fn `UserConstructionScript`)